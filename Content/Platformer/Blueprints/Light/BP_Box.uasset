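; BP_Box is a box actor that publishes the transform of its Cube component to materials through the PC_BoxData parameter collection.
; On BeginPlay it writes the cube's world location, its world scale as bounds, and its forward, right and up vectors as axes.
; The values are written only once, so later movement or resizing of the cube is not reflected in the collection.
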(event EventBeginPlay
  (bind _cube (Variables|Default|GetCube))
  (bind _cube_2 (Variables|Default|GetCube))
  (Rendering|Material|SetVectorParameterValue "/Game/Platformer/MaterialLibrary/Effects/PC_BoxData.PC_BoxData" "Location" (Math|Conversions|ToLinearColor(Vector) (Transformation|GetWorldLocation _cube)) :!class /Script/Engine.KismetMaterialLibrary)
  (Rendering|Material|SetVectorParameterValue "/Game/Platformer/MaterialLibrary/Effects/PC_BoxData.PC_BoxData" "Bounds" (Math|Conversions|ToLinearColor(Vector) (Transformation|GetWorldScale _cube)) :!class /Script/Engine.KismetMaterialLibrary)
  (Rendering|Material|SetVectorParameterValue "/Game/Platformer/MaterialLibrary/Effects/PC_BoxData.PC_BoxData" "X" (Math|Conversions|ToLinearColor(Vector) (Math|Vector|GetForwardVector _cube_2)) :!class /Script/Engine.KismetMaterialLibrary)
  (Rendering|Material|SetVectorParameterValue "/Game/Platformer/MaterialLibrary/Effects/PC_BoxData.PC_BoxData" "Y" (Math|Conversions|ToLinearColor(Vector) (Math|Vector|GetRightVector _cube_2)) :!class /Script/Engine.KismetMaterialLibrary)
  (Rendering|Material|SetVectorParameterValue "/Game/Platformer/MaterialLibrary/Effects/PC_BoxData.PC_BoxData" "z" (Math|Conversions|ToLinearColor(Vector) (Math|Vector|GetUpVector _cube_2)) :!class /Script/Engine.KismetMaterialLibrary))

(fn ConstructionScript)