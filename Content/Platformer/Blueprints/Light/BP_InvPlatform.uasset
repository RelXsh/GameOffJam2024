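; Invisible platform for a light-based platformer mechanic, whose Cube either blocks or ignores pawns.
; IsRevealed picks the dissolve or light-ray material and the Pawn collision response at construction, with collision reapplied on BeginPlay if revealed.
; SwitchState and LampSwitch flip both, while ToggleLight allows blocking only when revealed with the flashlight on.
; EndEffect drops pawn collision, and the old overlap logic is disconnected.
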(event OnComponentBeginOverlap(Cube)
  (params (OverlappedComponent :type Primitive%20Component%20Object%20Reference) (OtherActor :type Actor%20Object%20Reference) (OtherComp :type Primitive%20Component%20Object%20Reference) (OtherBodyIndex :type Integer) (bFromSweep :type Boolean) (SweepResult :type Hit%20Result%20Structure%20%28by%20ref%29))
  ;[1 1 1] OLD LOGIC - DO NOT USE
)

(event OnComponentEndOverlap(Cube)
  (params (OverlappedComponent :type Primitive%20Component%20Object%20Reference) (OtherActor :type Actor%20Object%20Reference) (OtherComp :type Primitive%20Component%20Object%20Reference) (OtherBodyIndex :type Integer))
  ;[1 1 1] OLD LOGIC - DO NOT USE
)

(event Custom|EndEffect
  ;[1 1 1] OLD LOGIC - DO NOT USE
  (Collision|SetCollisionResponsetoChannel (Variables|Default|GetCube) "ECC_Pawn" "ECR_Ignore"))

(event EventBeginPlay
  (if (Variables|Default|GetisRevealed)
    (Collision|SetCollisionResponsetoChannel (Variables|Default|GetCube) "ECC_Pawn" "ECR_Block")))

(event Collision|EventActorBeginOverlap
  (params (OtherActor :type Actor%20Object%20Reference)))

(event EventTick
  (params (DeltaSeconds :type Float%20%28single-precision%29)))

(fn ConstructionScript
  (bind _cube (Variables|Default|GetCube))
  (if (Variables|Default|GetisRevealed)
    (Rendering|Material|SetMaterial (Variables|Default|GetCube) 0 "/Game/Platformer/MaterialLibrary/Effects/M_InvDissolve.M_InvDissolve")
    (Collision|SetCollisionResponsetoChannel _cube "ECC_Pawn" "ECR_Block")
    (else
      (Rendering|Material|SetMaterial (Variables|Default|GetCube) 0 "/Game/Platformer/MaterialLibrary/Effects/M_lightRay.M_lightRay")
      (Collision|SetCollisionResponsetoChannel _cube "ECC_Pawn" "ECR_Ignore"))))

(fn SwitchState
  (bind _cube (Variables|Default|GetCube))
  (bind _cube_2 (Variables|Default|GetCube))
  (if (Variables|Default|GetisRevealed)
    (Variables|Default|SetisRevealed false)
    (Rendering|Material|SetMaterial _cube 0 "/Game/Platformer/MaterialLibrary/Effects/M_lightRay.M_lightRay")
    (Collision|SetCollisionResponsetoChannel _cube_2 "ECC_Pawn" "ECR_Ignore")
    (else
      (Variables|Default|SetisRevealed true)
      (Rendering|Material|SetMaterial _cube 0 "/Game/Platformer/MaterialLibrary/Effects/M_InvDissolve.M_InvDissolve")
      (Collision|SetCollisionResponsetoChannel _cube_2 "ECC_Pawn" "ECR_Block"))))

(fn ToggleLight
  (params (FlashlightOn%20 :type Boolean))
  (bind _isrevealed (Variables|Default|GetisRevealed))
  (bind _cube (Variables|Default|GetCube))
  (bind _cube_2 (Variables|Default|GetCube))
  (bind _output_get (Variables|Default|SetFlashLightOn FlashlightOn%20))
  (if _output_get
    (if _isrevealed
      (Collision|SetCollisionResponsetoChannel _cube "ECC_Pawn" "ECR_Block")
      (else
        (Collision|SetCollisionResponsetoChannel _cube "ECC_Pawn" "ECR_Ignore")))
    (elif _isrevealed
      (Collision|SetCollisionResponsetoChannel _cube_2 "ECC_Pawn" "ECR_Ignore")
      (else
        (Collision|SetCollisionResponsetoChannel _cube_2 "ECC_Pawn" "ECR_Ignore")))))

(fn LampSwitch
  (bind _cube (Variables|Default|GetCube))
  (if (Variables|Default|GetisRevealed)
    (Rendering|Material|SetMaterial (Variables|Default|GetCube) 0 "/Game/Platformer/MaterialLibrary/Effects/M_lightRay.M_lightRay")
    (Collision|SetCollisionResponsetoChannel _cube "ECC_Pawn" "ECR_Ignore")
    (else
      (Rendering|Material|SetMaterial (Variables|Default|GetCube) 0 "/Game/Platformer/MaterialLibrary/Effects/M_InvDissolve.M_InvDissolve")
      (Collision|SetCollisionResponsetoChannel _cube "ECC_Pawn" "ECR_Block")))
  (Variables|Default|SetisRevealed (not (Variables|Default|GetisRevealed))))