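; BP_Pickup is a flashlight pickup that destroys itself when BP_ThirdPersonCharacter overlaps its sphere.
; On overlap it overwrites the character's FlashlightCount, calls TurnOn and tints the character's SpotLight a fixed yellow.
; It then calls SwitchState on every entry in its InvToFlip and PlToFlip arrays.
; The construction script colors the pickup's PointLight from NewLightColor, which the spotlight tint ignores.
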(event OnComponentBeginOverlap(Sphere)
  (params (OverlappedComponent :type Primitive%20Component%20Object%20Reference) (OtherActor :type Actor%20Object%20Reference) (OtherComp :type Primitive%20Component%20Object%20Reference) (OtherBodyIndex :type Integer) (bFromSweep :type Boolean) (SweepResult :type Hit%20Result%20Structure%20%28by%20ref%29))
  (bind _asbp_third_person_character (Utilities|Casting|CastToBP_ThirdPersonCharacter OtherActor))
  (Variables|/Game/ThirdPerson/Blueprints/BP_ThirdPersonCharacter.BP_ThirdPersonCharacter_C|SetFlashlightCount _asbp_third_person_character (Variables|Default|GetFlashlight%20Count))
  (Development|PrintString "Hello")
  (Default|Turnon _asbp_third_person_character)
  (Rendering|Components|Light|SetLightColor (Variables|/Game/ThirdPerson/Blueprints/BP_ThirdPersonCharacter.BP_ThirdPersonCharacter_C|GetSpotLight _asbp_third_person_character) "(R=1.000000,G=0.983937,B=0.000000,A=1.000000)" true)
  (for _array_element (Variables|Default|GetInvToFlip)
    (Default|SwitchState _array_element))
  (for _array_element_2 (Variables|Default|GetplToFlip)
    (Default|SwitchState _array_element_2))
  (Actor|DestroyActor))

(event EventBeginPlay)

(event Collision|EventActorBeginOverlap
  (params (OtherActor :type Actor%20Object%20Reference)))

(event EventTick
  (params (DeltaSeconds :type Float%20%28single-precision%29)))

(fn ConstructionScript
  (Rendering|Components|Light|SetLightColor (Variables|Default|GetPointLight) (Variables|Default|GetNew%20Light%20Color) true))