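; Platform Blueprint for a platformer that toggles between a solid and a dissolved state, shown by swapping the Cube's material.
; The construction script sets the material from IsSolid, and SwitchState flips the flag and material without touching collision.
; Cube overlap events set the Pawn channel to Overlap when BP_ThirdPersonCharacter enters a non-solid platform, and back to Block when it leaves.
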(event OnComponentBeginOverlap(Cube)
  (params (OverlappedComponent :type Primitive%20Component%20Object%20Reference) (OtherActor :type Actor%20Object%20Reference) (OtherComp :type Primitive%20Component%20Object%20Reference) (OtherBodyIndex :type Integer) (bFromSweep :type Boolean) (SweepResult :type Hit%20Result%20Structure%20%28by%20ref%29))
  (Utilities|Casting|CastToBP_ThirdPersonCharacter OtherActor)
  (if (not (Variables|Default|GetisSolid))
    (Collision|SetCollisionResponsetoChannel (Variables|Default|GetCube) "ECC_Pawn" "ECR_Overlap")))

(event OnComponentEndOverlap(Cube)
  (params (OverlappedComponent :type Primitive%20Component%20Object%20Reference) (OtherActor :type Actor%20Object%20Reference) (OtherComp :type Primitive%20Component%20Object%20Reference) (OtherBodyIndex :type Integer))
  (Utilities|Casting|CastToBP_ThirdPersonCharacter OtherActor)
  (Collision|SetCollisionResponsetoChannel (Variables|Default|GetCube) "ECC_Pawn" "ECR_Block"))

(event EventBeginPlay)

(event Collision|EventActorBeginOverlap
  (params (OtherActor :type Actor%20Object%20Reference)))

(event EventTick
  (params (DeltaSeconds :type Float%20%28single-precision%29)))

(fn ConstructionScript
  (if (Variables|Default|GetisSolid)
    (Rendering|Material|SetMaterial (Variables|Default|GetCube) 0 "/Game/Platformer/MaterialLibrary/Effects/M_Solid.M_Solid")
    (else
      (Rendering|Material|SetMaterial (Variables|Default|GetCube) 0 "/Game/Platformer/MaterialLibrary/Effects/M_Dissolve.M_Dissolve"))))

(fn SwitchState
  (bind _output_get (Variables|Default|SetisSolid (not (Variables|Default|GetisSolid))))
  (if _output_get
    (Rendering|Material|SetMaterial (Variables|Default|GetCube) 0 "/Game/Platformer/MaterialLibrary/Effects/M_Solid.M_Solid")
    (else
      (Rendering|Material|SetMaterial (Variables|Default|GetCube) 0 "/Game/Platformer/MaterialLibrary/Effects/M_Dissolve.M_Dissolve"))))